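; Actor that moves a Cube along a rectangular path in the local X-Z plane, starting on BeginPlay.
; One timeline's four tracks, scaled by Distance, drive nested position checks against hardcoded thresholds to choose each leg.
; On finish, IsRight flips to alternate between Play and Reverse.
; The MoveType-based Move functions are an uncalled alternative, with their switch and input setup left unwired.
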(event `self.ReceiveBeginPlay`
  (bind _cube (`self.Cube`))
  (bind _cube_2 (`self.Cube`))
  (bind (_relativelocation_x _relativelocation_y _relativelocation_z) (`KismetMathLibrary.BreakVector` (`SceneComponent.RelativeLocation` _cube_2)))
  (bind _relativelocation_x_2 (`KismetMathLibrary.BreakVector` (`SceneComponent.RelativeLocation` _cube)))
  (bind _relativelocation_x_3 (`KismetMathLibrary.BreakVector` (`SceneComponent.RelativeLocation` (`self.Cube`))))
  (if (`self.IsRight`) :!label _label
    (bind (_direction _1 _2 _3 _4) (`Timeline|타임라인` :!label _label_2)
      (:`Update`
        (bind _returnvalue (* _1 (`self.Distance`)))
        (`SceneComponent.K2_SetRelativeLocation` _cube (`KismetMathLibrary.MakeVector` _returnvalue) false false)
        (if (>= _relativelocation_x_2 500.0)
          (`SceneComponent.K2_SetRelativeLocation` _cube (`KismetMathLibrary.MakeVector` _returnvalue 0.0 (* _2 (`self.Distance`))) false false)
          (if (>= _relativelocation_z 500.0)
            (`SceneComponent.K2_AddRelativeLocation` _cube_2 (`KismetMathLibrary.MakeVector` (* (* _3 (`self.Distance`)) -1.0)) false false)
            (if (<= _relativelocation_x_3 0.0)
              (`SceneComponent.K2_AddRelativeLocation` _cube_2 (`KismetMathLibrary.MakeVector` 0.0 0.0 (* (* _4 (`self.Distance`)) -1.0)) false false)
              (if (`KismetMathLibrary.EqualExactly_VectorVector` (`SceneComponent.RelativeLocation` (`self.Cube`)))
                _)))))
      (:`Finished`
        (set `self.IsRight` (not (`self.IsRight`)))
        (goto _label)))
    (else
      (goto _label_2 :!via `Reverse`))))

(fn `MoveDown`
  (params (A :type "Float (double-precision)"))
  (bind _cube (`self.Cube`))
  (bind (_relativelocation_x _relativelocation_y _relativelocation_z) (`KismetMathLibrary.BreakVector` (`SceneComponent.RelativeLocation` _cube)))
  (`SceneComponent.K2_SetRelativeLocation` _cube (`KismetMathLibrary.MakeVector` 0.0 0.0 (* A -1.0)) false false)
  (if (<= _relativelocation_z 0.0)
    (set `self.MoveType` "NewEnumerator0")))

(fn `MoveLeft`
  (params (A :type "Float (double-precision)"))
  (bind _cube (`self.Cube`))
  (bind _relativelocation_x (`KismetMathLibrary.BreakVector` (`SceneComponent.RelativeLocation` _cube)))
  (`SceneComponent.K2_SetRelativeLocation` _cube (`KismetMathLibrary.MakeVector` (* A -1.0) 0.0 (`self.Distance`)) false false)
  (if (<= _relativelocation_x 0.0)
    (set `self.MoveType` "NewEnumerator3")))

(fn `MoveRight`
  (params (DeltaLocation_X :type "Float (double-precision)"))
  (bind _cube (`self.Cube`))
  (bind _relativelocation_x (`KismetMathLibrary.BreakVector` (`SceneComponent.RelativeLocation` _cube)))
  (`SceneComponent.K2_SetRelativeLocation` _cube (`KismetMathLibrary.MakeVector` DeltaLocation_X) false false)
  (if (>= _relativelocation_x 500.0)
    (set `self.MoveType` "NewEnumerator1")))

(fn `MoveUp`
  (params (DeltaLocation_Z :type "Float (double-precision)"))
  (bind _cube (`self.Cube`))
  (bind (_relativelocation_x _relativelocation_y _relativelocation_z) (`KismetMathLibrary.BreakVector` (`SceneComponent.RelativeLocation` _cube)))
  (`SceneComponent.K2_SetRelativeLocation` _cube (`KismetMathLibrary.MakeVector` (`self.Distance`) 0.0 DeltaLocation_Z) false false)
  (if (>= _relativelocation_z 500.0)
    (set `self.MoveType` "NewEnumerator2")))

(fn `UserConstructionScript`)