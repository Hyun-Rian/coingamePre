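; BP_SwichBox is a switch that starts and stops a set of target actors when something overlaps its static mesh.
; Begin overlap sends EventPlayMessage, and end overlap sends EventStopMessage, to each entry in the Actors array that implements BPI_MoveActor.
; Both events also print a debug string, and neither filters which actor triggers the overlap.
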(event `self.StaticMesh.OnComponentBeginOverlap`
  (params (OverlappedComponent :type "PrimitiveComponent Object Reference") (OtherActor :type "Actor Object Reference") (OtherComp :type "PrimitiveComponent Object Reference") (OtherBodyIndex :type Integer) (bFromSweep :type Boolean) (SweepResult :type "HitResult Structure (by ref)"))
  (`KismetSystemLibrary.PrintString` "Move")
  (for _array_element (`self.Actors`)
    (if (`KismetSystemLibrary.DoesImplementInterface` _array_element "/Game/MyProject/BPI_MoveActor.BPI_MoveActor_C")
      (message `/Game/MyProject/BPI_MoveActor.EventPlay` _array_element))))

(event `self.StaticMesh.OnComponentEndOverlap`
  (params (OverlappedComponent :type "PrimitiveComponent Object Reference") (OtherActor :type "Actor Object Reference") (OtherComp :type "PrimitiveComponent Object Reference") (OtherBodyIndex :type Integer))
  (`KismetSystemLibrary.PrintString` "Stop")
  (for _array_element (`self.Actors`)
    (if (`KismetSystemLibrary.DoesImplementInterface` _array_element "/Game/MyProject/BPI_MoveActor.BPI_MoveActor_C")
      (message `/Game/MyProject/BPI_MoveActor.EventStop` _array_element))))

(fn `UserConstructionScript`)