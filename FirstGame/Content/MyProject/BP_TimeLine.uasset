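; BP_TimeLine is a timeline-driven actor that slides its Cube back and forth along the relative X axis.
; EventPlay plays or reverses the timeline based on IsRight, with the track value scaled by Distance setting the cube's X position.
; When the timeline finishes, IsRight flips and playback repeats in the other direction until EventStop halts it.
; BeginPlay enables input for player 0, though no input events appear in the graph.
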(event `self.ReceiveBeginPlay`
  (`self.EnableInput` (`GameplayStatics.GetPlayerController` 0)))

(event `/Game/MyProject/BPI_MoveActor.EventPlay`
  (if (`self.IsRight`) :!label _label
    (bind (_direction `_새_트랙_0`) (`Timeline|타임라인` :`NewTime` 0.5 :!label _label_2)
      (:`Update`
        (`SceneComponent.K2_SetRelativeLocation` (`self.Cube`) (`KismetMathLibrary.MakeVector` (* `_새_트랙_0` (`self.Distance`))) false false))
      (:`Finished`
        (set `self.IsRight` (not (`self.IsRight`)))
        (goto _label)))
    (else
      (goto _label_2 :!via `Reverse`))))

(event `/Game/MyProject/BPI_MoveActor.EventStop`
  (goto _label_2 :!via `Stop`))

(event `Key|P`
  (params (Key :type "Key Structure")))

(fn `UserConstructionScript`)