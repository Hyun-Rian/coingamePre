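; Actor that slides its static mesh back and forth along its local X axis, like a simple moving platform.
; While play is enabled, Tick adds a Speed-scaled, frame-rate-independent offset and flips direction at fixed limits at either end.
; EventPlay and EventStop toggle the movement on and off.
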(event `self.ReceiveTick`
  (params (DeltaSeconds :type "Float (single-precision)"))
  (bind _staticmesh (`self.StaticMesh`))
  (bind _staticmesh_2 (`self.StaticMesh`))
  (bind _returnvalue (* DeltaSeconds (`self.speed`)))
  (bind _relativelocation_x (`KismetMathLibrary.BreakVector` (`SceneComponent.RelativeLocation` _staticmesh)))
  (bind _relativelocation_x_2 (`KismetMathLibrary.BreakVector` (`SceneComponent.RelativeLocation` _staticmesh_2)))
  (if (`self.Isplay`)
    (if (`self.MoveRight`)
      (`SceneComponent.K2_AddRelativeLocation` _staticmesh_2 (`KismetMathLibrary.MakeVector` _returnvalue) false false)
      (if (>= _relativelocation_x_2 500.0)
        (set `self.MoveRight` false))
      (else
        (`SceneComponent.K2_AddRelativeLocation` _staticmesh (`KismetMathLibrary.MakeVector` (* _returnvalue -1.0)) false false)
        (if (<= _relativelocation_x 0.0)
          (set `self.MoveRight` true))))))

(event `/Game/MyProject/BPI_MoveActor.EventPlay`
  (set `self.Isplay` true))

(event `/Game/MyProject/BPI_MoveActor.EventStop`
  (set `self.Isplay` false))

(fn `UserConstructionScript`)