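; BP_CoinH is a collectible coin actor that spins and notifies other objects when picked up.
; It starts hidden with collision disabled on BeginPlay, with nothing in this Blueprint re-enabling it.
; Tick adds a small fixed rotation to the Coin component each frame, independent of delta time.
; An overlap on Coin destroys the actor and fires events on PotalH and CoinCounterH to register the pickup.
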(event `self.ReceiveBeginPlay`
  (`self.SetActorHiddenInGame` true)
  (`self.SetActorEnableCollision` false))

(event `self.ReceiveTick`
  (params (DeltaSeconds :type "Float (single-precision)"))
  (`SceneComponent.K2_AddRelativeRotation` (`self.Coin`) (struct :`Yaw` 1.0) false false))

(event `self.Coin.OnComponentBeginOverlap`
  (params (OverlappedComponent :type "PrimitiveComponent Object Reference") (OtherActor :type "Actor Object Reference") (OtherComp :type "PrimitiveComponent Object Reference") (OtherBodyIndex :type Integer) (bFromSweep :type Boolean) (SweepResult :type "HitResult Structure (by ref)"))
  (`self.K2_DestroyActor`)
  (`/Game/MyProject/Coin_Game/Coin_GameH/BP_PotalH.Event Coin Overlap` (`self.Potal H`))
  (`/Game/MyProject/Coin_Game/Coin_GameH/BP_CoinCounterH.Event Count Coin` (`self.CoinCounterH`)))

(fn `UserConstructionScript`)