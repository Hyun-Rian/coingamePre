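; BP_GameStateBase is a game state Blueprint that runs an elapsed-time clock and shows it on the HUD.
; Each Tick, PrintTime adds delta time scaled to run ten times faster than real time to TotalSecond.
; It splits the total into minutes and seconds, zero-pads each through GetFloatToStr00, and passes the joined text to BP_HUD via the first player controller.
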(event `self.ReceiveTick`
  (params (DeltaSeconds :type "Float (single-precision)"))
  (`self.PrintTime` DeltaSeconds))

(fn `getFloatToStr00`
  (params (number :type "Float (double-precision)"))
  (returns (Str00 :type String))
  (bind _returnvalue (`KismetStringLibrary.Conv_IntToString` (`KismetMathLibrary.FFloor` number)))
  (if (< number 10.0)
    (return (`KismetStringLibrary.Concat_StrStr` "0" _returnvalue))
    (else
      (return _returnvalue))))

(fn `PrintTime`
  (params (DeltaSecond :type "Float (double-precision)"))
  (bind _output_get (set `self.TotalSecond` (+ (`self.TotalSecond`) (* DeltaSecond 10.0))))
  (bind _asbp_hud (cast `/Game/MyProject/Coin_Game/Coin_GameH/5Day/GameMode/BP_HUD` (`PlayerController.GetHUD` (`GameplayStatics.GetPlayerController` 0))))
  (`/Game/MyProject/Coin_Game/Coin_GameH/5Day/GameMode/BP_HUD.SetTimeText` _asbp_hud (`KismetStringLibrary.Concat_StrStr` (`self.getFloatToStr00` (/ _output_get 60.0)) ":" (`self.getFloatToStr00` (mod _output_get 60.0)))))

(fn `UserConstructionScript`)