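; Player state for a coin game that tracks the player's coin count and red, green, blue and black item counts.
; Add functions increment a count and push it to BP_HUD through player controller 0's HUD.
; Use functions decrement only when stock remains, update the HUD and return success.
; Only the red item prints an out-of-stock message, and UseBlackItem's false return node is left unconnected.
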(fn `AddBlackItem`
  (bind _output_get (set `self.BlackItem` (+ (`self.BlackItem`) 1)))
  (bind _asbp_hud (cast `/Game/MyProject/Coin_Game/Coin_GameH/5Day/GameMode/BP_HUD` (`PlayerController.GetHUD` (`GameplayStatics.GetPlayerController` 0))))
  (`/Game/MyProject/Coin_Game/Coin_GameH/5Day/GameMode/BP_HUD.SetBlackItemText` _asbp_hud _output_get))

(fn `AddBuleItem`
  (bind _output_get (set `self.BuleItem` (+ (`self.BuleItem`) 1)))
  (bind _asbp_hud (cast `/Game/MyProject/Coin_Game/Coin_GameH/5Day/GameMode/BP_HUD` (`PlayerController.GetHUD` (`GameplayStatics.GetPlayerController` 0))))
  (`/Game/MyProject/Coin_Game/Coin_GameH/5Day/GameMode/BP_HUD.SetBuleItemText` _asbp_hud _output_get))

(fn `AddCoin`
  (bind _output_get (set `self.Coin` (+ (`self.Coin`) 1)))
  (bind _asbp_hud (cast `/Game/MyProject/Coin_Game/Coin_GameH/5Day/GameMode/BP_HUD` (`PlayerController.GetHUD` (`GameplayStatics.GetPlayerController` 0))))
  (`/Game/MyProject/Coin_Game/Coin_GameH/5Day/GameMode/BP_HUD.SetCoinText` _asbp_hud _output_get))

(fn `AddGreenItem`
  (bind _output_get (set `self.GreenItem` (+ (`self.GreenItem`) 1)))
  (bind _asbp_hud (cast `/Game/MyProject/Coin_Game/Coin_GameH/5Day/GameMode/BP_HUD` (`PlayerController.GetHUD` (`GameplayStatics.GetPlayerController` 0))))
  (`/Game/MyProject/Coin_Game/Coin_GameH/5Day/GameMode/BP_HUD.SetGreenItemText` _asbp_hud _output_get))

(fn `AddRedItem`
  (bind _output_get (set `self.RedItem` (+ (`self.RedItem`) 1)))
  (bind _asbp_hud (cast `/Game/MyProject/Coin_Game/Coin_GameH/5Day/GameMode/BP_HUD` (`PlayerController.GetHUD` (`GameplayStatics.GetPlayerController` 0))))
  (`/Game/MyProject/Coin_Game/Coin_GameH/5Day/GameMode/BP_HUD.SetRedItemText` _asbp_hud _output_get))

(fn `UseBlackItem`
  (returns (IsUsed :type Boolean))
  (bind _blackitem (`self.BlackItem`))
  (if (> _blackitem 0)
    (bind _output_get (set `self.BlackItem` (- _blackitem 1)))
    (bind _asbp_hud (cast `/Game/MyProject/Coin_Game/Coin_GameH/5Day/GameMode/BP_HUD` (`PlayerController.GetHUD` (`GameplayStatics.GetPlayerController` 0))))
    (`/Game/MyProject/Coin_Game/Coin_GameH/5Day/GameMode/BP_HUD.SetBlackItemText` _asbp_hud _output_get)
    (return true)))

(fn `UseBuleItem`
  (returns (Isused :type Boolean))
  (bind _buleitem (`self.BuleItem`))
  (if (> _buleitem 0)
    (bind _output_get (set `self.BuleItem` (- _buleitem 1)))
    (bind _asbp_hud (cast `/Game/MyProject/Coin_Game/Coin_GameH/5Day/GameMode/BP_HUD` (`PlayerController.GetHUD` (`GameplayStatics.GetPlayerController` 0))))
    (`/Game/MyProject/Coin_Game/Coin_GameH/5Day/GameMode/BP_HUD.SetBuleItemText` _asbp_hud _output_get)
    (return true)
    (else
      (return false))))

(fn `UseGreenItem`
  (returns (IsUsed :type Boolean))
  (if (> (`self.GreenItem`) 0)
    (bind _output_get (set `self.GreenItem` (- (`self.GreenItem`) 1)))
    (bind _asbp_hud (cast `/Game/MyProject/Coin_Game/Coin_GameH/5Day/GameMode/BP_HUD` (`PlayerController.GetHUD` (`GameplayStatics.GetPlayerController` 0))))
    (`/Game/MyProject/Coin_Game/Coin_GameH/5Day/GameMode/BP_HUD.SetGreenItemText` _asbp_hud _output_get)
    (return true)
    (else
      (return false))))

(fn `UserConstructionScript`)

(fn `UseRedItem`
  (returns (IsUsed :type Boolean))
  (if (> (`self.RedItem`) 0)
    (bind _output_get (set `self.RedItem` (- (`self.RedItem`) 1)))
    (bind _asbp_hud (cast `/Game/MyProject/Coin_Game/Coin_GameH/5Day/GameMode/BP_HUD` (`PlayerController.GetHUD` (`GameplayStatics.GetPlayerController` 0))))
    (`/Game/MyProject/Coin_Game/Coin_GameH/5Day/GameMode/BP_HUD.SetRedItemText` _asbp_hud _output_get)
    (return true)
    (else
      (`KismetSystemLibrary.PrintString` "아이템이 없어!")
      (return false))))