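; BP_MoveSpilne is an actor that moves its Cube back and forth along a Spline component from BeginPlay onward.
; A timeline track scales the spline length into a distance, and each update places the Cube at that world-space location without sweep.
; When the timeline finishes, IsRight flips and selects Play or Reverse, creating an endless ping-pong loop.
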(event `self.ReceiveBeginPlay`
  (if (`self.IsRight`) :!label _label
    (bind (_direction `_새_트랙_0`) (`Timeline|타임라인` :!label _label_2)
      (:`Update`
        (`SceneComponent.K2_SetWorldLocation` (`self.Cube`) (`SplineComponent.GetLocationAtDistanceAlongSpline` (`self.Spline`) (* `_새_트랙_0` (`SplineComponent.GetSplineLength` (`self.Spline`))) "World") false false))
      (:`Finished`
        (set `self.IsRight` (not (`self.IsRight`)))
        (goto _label)))
    (else
      (goto _label_2 :!via `Reverse`))))

(fn `UserConstructionScript`)