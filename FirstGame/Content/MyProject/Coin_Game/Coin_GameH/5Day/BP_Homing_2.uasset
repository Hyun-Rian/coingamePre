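; BP_Homing_2 is a homing projectile that chases the player character in the coin game.
; While the game state is Play, Tick moves it along its Arrow's forward vector at a fixed per-frame step and eases its rotation toward the player with RInterpTo.
; Any sphere overlap makes it explode and destroy itself; hitting BP_ThirdPersonCharacter1 also adds damage through BP_PlayerState and triggers ragdoll.
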(event `self.ReceiveTick`
  (params (DeltaSeconds :type "Float (single-precision)"))
  (if (`self.IsCanMove`)
    (`/Engine/EditorBlueprintResources/StandardMacros.IsValid` (`self.HomingTarget`)
      (:`Is Valid`
        (`self.K2_AddActorWorldOffset` (* (`SceneComponent.GetForwardVector` (`self.Arrow`)) 5.0))
        (`self.K2_SetActorRotation` (`KismetMathLibrary.RInterpTo` (`self.K2_GetActorRotation`) (`KismetMathLibrary.FindLookAtRotation` (`self.K2_GetActorLocation`) (`self.K2_GetActorLocation` (`self.HomingTarget`))) DeltaSeconds 2.0))))))

(event `self.ReceiveBeginPlay`
  (set `self.HomingTarget` (`GameplayStatics.GetPlayerCharacter` 0))
  (bind _asbp_game_state_base (cast `/Game/MyProject/Coin_Game/Coin_GameH/5Day/GameMode/BP_GameStateBase` (`GameplayStatics.GetGameState`)))
  (add `/Game/MyProject/Coin_Game/Coin_GameH/5Day/GameMode/BP_GameStateBase.EventDispatcher_ChangeGameState` _asbp_game_state_base (`|CreateDelegate` :!event `PlayMoveHoming`)))

(event `self.Sphere.OnComponentBeginOverlap`
  (params (OverlappedComponent :type "PrimitiveComponent Object Reference") (OtherActor :type "Actor Object Reference") (OtherComp :type "PrimitiveComponent Object Reference") (OtherBodyIndex :type Integer) (bFromSweep :type Boolean) (SweepResult :type "HitResult Structure (by ref)"))
  (`self.EventHitCharater` OtherActor)
  (`self.Destory Homing`))

(fn `Destory Homing`
  (`GameplayStatics.SpawnEmitterAtLocation` "/Game/StarterContent/Particles/P_Explosion.P_Explosion" (`self.K2_GetActorLocation`) (`self.K2_GetActorRotation`) (2.0 2.0 2.0))
  (`self.K2_DestroyActor`))

(fn `EventHitCharater`
  (params (actor :type "Actor Object Reference"))
  (bind _asbp_third_person_character_1 (cast `/Game/MyProject/Coin_Game/Coin_GameH/5Day/GameMode/BP_ThirdPersonCharacter1` actor))
  (bind _asbp_player_state (cast `/Game/MyProject/Coin_Game/Coin_GameH/5Day/GameMode/BP_PlayerState` (`Pawn.PlayerState` _asbp_third_person_character_1)))
  (`/Game/MyProject/Coin_Game/Coin_GameH/5Day/GameMode/BP_PlayerState.Add Damage` _asbp_player_state 10.0)
  (`/Game/MyProject/Coin_Game/Coin_GameH/5Day/GameMode/BP_ThirdPersonCharacter1.DoRagdoll` _asbp_third_person_character_1))

(fn `PlayMoveHoming`
  (params (GameState :type "/Game/MyProject/Coin_Game/Coin_GameH/5Day/GameMode/EN_GameState Enum" :default "NewEnumerator3"))
  (switch `/Game/MyProject/Coin_Game/Coin_GameH/5Day/GameMode/EN_GameState` GameState
    (:`NewEnumerator3`
      (set `self.IsCanMove` false :!label _label))
    (:`NewEnumerator0`
      (goto _label))
    (:`NewEnumerator1`
      (set `self.IsCanMove` true))))

(fn `UserConstructionScript`)