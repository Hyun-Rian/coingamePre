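; Portal actor for the coin game that stays hidden and non-collidable until all coins are collected.
; EventCoinOverlap calls IsGetAllCoin, which scans the level for valid BP_CoinH actors, and turns on the mesh's visibility and collision when none remain.
; Overlapping the revealed mesh calls EventOverlapPotal on the referenced BPTeleportpoint.
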(event `self.ReceiveBeginPlay`
  (`SceneComponent.SetVisibility` (`self.StaticMesh`) false false)
  (`PrimitiveComponent.SetCollisionEnabled` (`self.StaticMesh`) "NoCollision"))

(event `self.StaticMesh.OnComponentBeginOverlap`
  (params (OverlappedComponent :type "PrimitiveComponent Object Reference") (OtherActor :type "Actor Object Reference") (OtherComp :type "PrimitiveComponent Object Reference") (OtherBodyIndex :type Integer) (bFromSweep :type Boolean) (SweepResult :type "HitResult Structure (by ref)"))
  (`/Game/MyProject/Coin_Game/Coin_GameH/BP_TeleportPointSetH.Event Overlap Potal` (`self.BP_teleportpoint`)))

(fn `Event Coin Overlap`
  (bind _isgetall (`self.IsGetAllCoin`))
  (if _isgetall
    (`SceneComponent.SetVisibility` (`self.StaticMesh`) true false)
    (`PrimitiveComponent.SetCollisionEnabled` (`self.StaticMesh`) "QueryAndPhysics")))

(fn `IsGetAllCoin`
  (returns (IsGetAll :type Boolean))
  (bind _outactors (`GameplayStatics.GetAllActorsOfClass` "/Game/MyProject/Coin_Game/Coin_GameH/BP_CoinH.BP_CoinH_C"))
  (for _array_element _outactors
    (`/Engine/EditorBlueprintResources/StandardMacros.IsValid` _array_element
      (:`Is Valid`
        (return false))))
  (return true))

(fn `UserConstructionScript`)